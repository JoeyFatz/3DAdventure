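; DialogueTrigger_BP shows and hides two dialogue widgets through a pair of trigger events, one per dialogue.
; Each event checks its Interaction flag: when true, it creates the matching widget, stores a reference and adds it to the viewport.
; When false, it finds top-level widgets of that class and removes them instead of using the stored reference.
; The flags are not set within this graph.
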(event `self.TriggerDialogue01`
  (if (`self.bInteraction01`)
    (bind _returnvalue (`|CreateWidget` "/Game/Blueprints/Widgets/DialogueOverlays/Dialogue_01_Widget.Dialogue_01_Widget_C"))
    (bind _output_get (set `self.DialogueOne` _returnvalue))
    (`UserWidget.AddToViewport` _output_get 0)
    (else
      (bind _foundwidgets (`WidgetBlueprintLibrary.GetAllWidgetsOfClass` "/Game/Blueprints/Widgets/DialogueOverlays/Dialogue_01_Widget.Dialogue_01_Widget_C"))
      (`Widget.RemoveFromParent` _foundwidgets))))

(event `self.TriggerDialogue02`
  (if (`self.bInteraction02`)
    (bind _returnvalue (`|CreateWidget` "/Game/Blueprints/Widgets/DialogueOverlays/Dialogue_02_Widget.Dialogue_02_Widget_C"))
    (bind _output_get (set `self.DialogueTwo` _returnvalue))
    (`UserWidget.AddToViewport` _output_get 0)
    (else
      (bind _foundwidgets (`WidgetBlueprintLibrary.GetAllWidgetsOfClass` "/Game/Blueprints/Widgets/DialogueOverlays/Dialogue_02_Widget.Dialogue_02_Widget_C"))
      (`Widget.RemoveFromParent` _foundwidgets))))

(fn `UserConstructionScript`)